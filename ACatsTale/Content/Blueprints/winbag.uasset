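; An overlap-triggered actor, winbag, that shows a CatThoughts dialogue widget when the ThirdPersonCharacter touches it.
; On overlap it creates the widget, passes it the Dialogue array as Lines, displays the first line and adds it to the viewport.
; A trailing cast of the player character feeds no further logic, and nothing here guards against repeated overlaps creating new widgets.
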(event EventBeginPlay)

(event Collision|EventActorBeginOverlap
  (params (OtherActor :type Actor%20Object%20Reference))
  (bind _dialogue (Variables|Default|GetDialogue))
  (Utilities|Casting|CastToThirdPersonCharacter OtherActor)
  (bind _returnvalue (UserInterface|CreateWidget "/Game/Blueprints/UI/CatThoughts.CatThoughts_C"))
  (bind _output_get (Variables|Default|Setwdij _returnvalue))
  (Variables|/Game/Blueprints/UI/CatThoughts.CatThoughts_C|SetLines _output_get _dialogue)
  (Rendering|Components|TextRender|SetText (Variables|/Game/Blueprints/UI/CatThoughts.CatThoughts_C|GetDiaText _output_get) (Utilities|Array|Get(acopy) _dialogue))
  (UserInterface|Viewport|AddtoViewport _output_get 0)
  (Utilities|Casting|CastToThirdPersonCharacter (Game|GetPlayerCharacter 0)))

(event EventTick
  (params (DeltaSeconds :type Float%20%28single-precision%29)))

(fn ConstructionScript)