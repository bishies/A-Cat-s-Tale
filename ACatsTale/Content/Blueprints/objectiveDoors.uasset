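; Objective door actor that swings open, once only, when its DoorOpenE event is called.
; The construction script stores the root's world rotation as closed and derives the open rotation 90 degrees lower in yaw.
; A timeline drives RInterpTo from the fixed closed rotation, feeding its track in as DeltaTime rather than frame time.
; Tick also accumulates a scaled Time value, which the door motion does not use.
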(event Custom|DoorOpenE
  (Utilities|FlowControl|DoOnce false
    (:Completed
      (bind _newtrack_0 (Timeline|DoorOpen PlayFromStart)
        (:Update
          (Transformation|SetWorldRotation (Variables|Default|GetScene) (Math|Interpolation|RInterpTo (Variables|Default|GetClosedRotation) (Variables|Default|GetOpenRotation) _newtrack_0 0.05) false false))))))

(event EventBeginPlay)

(event Collision|EventActorBeginOverlap
  (params (OtherActor :type Actor%20Object%20Reference)))

(event EventTick
  (params (DeltaSeconds :type Float%20%28single-precision%29))
  (Variables|Default|SetTime (+ (* DeltaSeconds (Variables|Default|GetRate)) (Variables|Default|GetTime))))

(fn ConstructionScript
  (bind _output_get (Variables|Default|SetClosedRotation (Transformation|GetWorldRotation (Variables|Default|GetScene))))
  (Variables|Default|SetOpenRotation (Math|Rotator|MakeRotator (.roll _output_get) (.pitch _output_get) (- (.yaw _output_get) 9e+01))))