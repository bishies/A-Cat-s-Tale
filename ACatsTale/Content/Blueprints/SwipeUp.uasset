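; SwipeUp is a short-lived actor that travels along a set direction and destroys itself at a height limit.
; BeginPlay stores an end point from its start location plus OffsetLimit.
; Each Tick teleport-free, unswept transform updates advance it from the Sphere's transform by normalized Direction, Speed and delta time, until its Z reaches that end point.
; A disconnected spawn snippet for SwipeUp remains in the graph.
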(event Collision|EventActorBeginOverlap
  (params (OtherActor :type Actor%20Object%20Reference)))

(event EventTick
  (params (DeltaSeconds :type Float%20%28single-precision%29))
  (bind _sphere (Variables|Default|GetSphere))
  (bind _returnvalue (Transformation|GetWorldTransform _sphere))
  (bind (_location _rotation _scale) (Math|Transform|BreakTransform _returnvalue))
  (Transformation|SetActorTransform (Math|Transform|MakeTransform (+ (* (Math|Vector|Normalize (Variables|Default|Getdirection)) (* (Utilities|Time|GetWorldDeltaSeconds) (Variables|Default|Getspeed))) _location) _rotation _scale))
  (if (>= (.Z (Math|Vector|BreakVector (Transformation|GetActorLocation))) (.Z (Math|Vector|BreakVector (Variables|Default|Getfinal%20location))))
    (Actor|DestroyActor)))

(event EventBeginPlay
  (Variables|Default|Setfinal%20location (+ (Transformation|GetActorLocation) (Variables|Default|Getoffset%20limit))))

(fn ConstructionScript)