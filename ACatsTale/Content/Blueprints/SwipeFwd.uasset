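; SwipeFwd is an actor that travels horizontally along the player's facing direction, likely as a forward swipe.
; On the first Tick, it caches the player's location and uses yaw trigonometry to project a target point DistanceTravel ahead.
; Each Tick moves it along that fixed direction at Speed, scaled by delta time, using the Sphere's transform without sweeping.
; It destroys itself when its squared XY distance from the target reaches DistanceTravel squared or more.
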(event Collision|EventActorBeginOverlap
  (params (OtherActor :type Actor%20Object%20Reference)))

(event EventTick
  (params (DeltaSeconds :type Float%20%28single-precision%29))
  (bind _returnvalue (Transformation|GetActorLocation))
  (bind _sphere (Variables|Default|GetSphere))
  (bind (_x _y) (Math|Vector|BreakVector _returnvalue))
  (bind _returnvalue_2 (Transformation|GetWorldTransform _sphere))
  (bind (_location _rotation _scale) (Math|Transform|BreakTransform _returnvalue_2))
  (Utilities|FlowControl|Sequence
    (:then_0
      (Utilities|FlowControl|DoOnce false
        (:Completed
          (Variables|Default|SetPlayer%20Yaw (.Yaw (Math|Rotator|BreakRotator (Transformation|GetActorRotation (Variables|Default|Getplayer)))))
          (Variables|Default|SetPlayer%20location (Transformation|GetActorLocation (Variables|Default|Getplayer)))
          (Variables|Default|Setfinal%20location (Math|Vector|MakeVector (+ (* (Math|Trig|Cos(Degrees) (Variables|Default|GetPlayer%20Yaw)) (Variables|Default|Getdistance%20travel)) (.X (Math|Vector|BreakVector (Variables|Default|GetPlayer%20location)))) (+ (.Y (Math|Vector|BreakVector (Variables|Default|GetPlayer%20location))) (* (Math|Trig|Sin(Degrees) (Variables|Default|GetPlayer%20Yaw)) (Variables|Default|Getdistance%20travel))) 0.0)))))
    (:then_1
      (Transformation|SetActorTransform (Math|Transform|MakeTransform (+ (* (Math|Vector|Normalize (Math|Vector|MakeVector (- (.X (Math|Vector|BreakVector (Variables|Default|Getfinal%20location))) (.X (Math|Vector|BreakVector (Variables|Default|GetPlayer%20location)))) (- (.Y (Math|Vector|BreakVector (Variables|Default|Getfinal%20location))) (.Y (Math|Vector|BreakVector (Variables|Default|GetPlayer%20location)))) 0.0)) (* (Utilities|Time|GetWorldDeltaSeconds) (Variables|Default|Getspeed))) _location) _rotation _scale))
      (if (>= (+ (Math|Float|Square (- (.X (Math|Vector|BreakVector (Variables|Default|Getfinal%20location))) _x)) (Math|Float|Square (- (.Y (Math|Vector|BreakVector (Variables|Default|Getfinal%20location))) _y))) (Math|Float|Square (Variables|Default|Getdistance%20travel)))
        (Actor|DestroyActor)))))

(fn ConstructionScript)